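; BP_Grappeling draws the lightning beam effect for the principal character's grapple, with no movement logic of its own.
; UseGrappeling stores the mesh, socket and target actor, then spawns the PS_Lightning emitter at the socket.
; Tick pins each beam's source to the socket and its end to the target, collapsing onto the socket if the target is invalid.
; Randomly delayed tangent changes on random emitters make the beam wiggle.
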(event EventTick
  (params (DeltaSeconds :type Float%20%28single-precision%29))
  (bind _ps_lightning (Variables|Default|GetPS_Lightning)
    (:then
      (for _index (range 0 (- (Class|ParticleSystemComponent|GetNumActiveParticles _ps_lightning) 1))
        ;[1 1 1] Set Source and Target
        (Variables|Default|SetParticleIndex _index)
        (Class|ParticleSystemComponent|SetBeamSourcePoint (Variables|Default|GetPS_Lightning) (Variables|Default|GetParticleIndex) (Transformation|GetSocketLocation (Variables|Default|GetSourceMesh) (Variables|Default|GetSocketSource)))
        (bind _target (Variables|Default|GetTarget)
          (:then
            (Variables|Default|SetTargetPoint (Transformation|GetActorLocation _target)))
          (:else
            (Variables|Default|SetTargetPoint (Transformation|GetSocketLocation (Variables|Default|GetSourceMesh) (Variables|Default|GetSocketSource)))))
        (Class|ParticleSystemComponent|SetBeamTargetPoint (Variables|Default|GetPS_Lightning) (Variables|Default|GetParticleIndex) (Variables|Default|GetTargetPoint)))
      ;[1 1 1] Wiggle beam tangent
      (Utilities|FlowControl|Sequence
        (:then_0
          (Utilities|FlowControl|Delay (Math|Random|RandomFloatinRange 0.1 0.5))
          (Class|ParticleSystemComponent|SetBeamSourceTangent (Variables|Default|GetPS_Lightning) (Math|Random|RandomIntegerinRange 0 (- (Class|ParticleSystemComponent|GetNumActiveParticles (Variables|Default|GetPS_Lightning)) 1)) (Math|Vector|MakeVector 0.0 (Math|Random|RandomFloatinRange -3e+01 3e+01) (Math|Random|RandomFloatinRange -3e+01 3e+01))))
        (:then_1
          (Utilities|FlowControl|Delay (Math|Random|RandomFloatinRange 0.1 0.5))
          (Class|ParticleSystemComponent|SetBeamTargetTangent (Variables|Default|GetPS_Lightning) (Math|Random|RandomIntegerinRange 0 (- (Class|ParticleSystemComponent|GetNumActiveParticles (Variables|Default|GetPS_Lightning)) 1)) (Math|Vector|MakeVector 0.0 (Math|Random|RandomFloatinRange -3e+01 3e+01) (Math|Random|RandomFloatinRange -3e+01 3e+01))))))
    (:else)))

(fn UseGrappeling
  (params (Mesh :type Skeletal%20Mesh%20Component%20Object%20Reference) (SocketSource :type Name) (TargetPoint :type Actor%20Object%20Reference))
  (Variables|Default|SetSourceMesh Mesh)
  (Variables|Default|SetSocketSource SocketSource)
  (Variables|Default|SetTarget TargetPoint)
  (bind _returnvalue (Effects|SpawnEmitteratLocation "/Game/ParticleSystem/PS_Lightning.PS_Lightning" (Transformation|GetSocketLocation (Variables|Default|GetSourceMesh) (Variables|Default|GetSocketSource))))
  (Variables|Default|SetPS_Lightning _returnvalue))