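; Grappling hook actor that links a character's mesh socket to a grabbed target with wiggling lightning beams and can throw that target at another actor.
; Grab binds the target to the root capsule through a physics constraint and enables physics simulation.
; After Throw, Tick rebuilds a distance-scaled spline and a timeline moves the capsule along it, dragging the target.
; Hitting anything but the owner ends the throw, keeping or dropping the target.
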(event Custom|OnTargetHit
  (params (SelfActor :type Actor%20Object%20Reference) (OtherActor :type Actor%20Object%20Reference) (NormalImpulse :type Vector) (Hit :type Hit%20Result%20Structure%20%28by%20ref%29))
  (if (!= OtherActor (Components|GetOwner (Variables|Particle|Source|GetSourceMesh)))
    (Rendering|Debug|DrawDebugPoint (Transformation|GetActorLocation (Variables|Particle|Target|GetTarget)) 25.0 "(R=1.000000,G=0.000000,B=0.000000,A=1.000000)" 2.5e+02)
    (Utilities|FlowControl|Sequence
      (:then_0
        (Utilities|KeeporDrop
          (:Keep
            (Transformation|SetActorRelativeLocation "0, 0,0.000000"))
          (:Drop
            (Variables|Particle|Target|SetTarget 0)
            (Class|PhysicsConstraintComponent|SetConstrainedComponents (Variables|Default|GetPhysicsConstraint) (Variables|Default|GetRootCapsule) "None" 0 "None"))))
      (:then_1
        (EventDispatchers|UnbindallEventsfromOnActorHit (Variables|Particle|Target|GetTarget))
        (Variables|Throw|SetTargetLaunch 0)))))

(event Custom|ResetDoOnceThrow
  ;[1 1 1] Throw object
  (Utilities|FlowControl|DoOnce false) ; enters at Reset
)

(event EventTick
  (params (DeltaSeconds :type Float%20%28single-precision%29))
  (bind _spline (Variables|Default|GetSpline))
  (for _index (range 0 (- (Class|ParticleSystemComponent|GetNumActiveParticles (Variables|Default|GetPS_Lightning)) 1))
    ;[1 1 1] Set Source and Target
    (Variables|Particle|Default|SetParticleIndex _index)
    (Class|ParticleSystemComponent|SetBeamSourcePoint (Variables|Default|GetPS_Lightning) (Variables|Particle|Default|GetParticleIndex) (Transformation|GetSocketLocation (Variables|Particle|Source|GetSourceMesh) (Variables|Particle|Source|GetSocketSource)))
    (bind _target (Variables|Particle|Target|GetTarget)
      (:then
        (Variables|Particle|Target|SetTargetPoint (Transformation|GetActorLocation _target)))
      (:else
        (Variables|Particle|Target|SetTargetPoint (Transformation|GetSocketLocation (Variables|Particle|Source|GetSourceMesh) (Variables|Particle|Source|GetSocketSource)))))
    (Class|ParticleSystemComponent|SetBeamTargetPoint (Variables|Default|GetPS_Lightning) (Variables|Particle|Default|GetParticleIndex) (Variables|Particle|Target|GetTargetPoint)))
  (Utilities|FlowControl|Sequence
    (:then_0
      ;[1 1 1] Wiggle beam tangent
      (Utilities|FlowControl|Sequence
        (:then_0
          (Utilities|FlowControl|Delay (Math|Random|RandomFloatinRange 0.1 0.5))
          (Class|ParticleSystemComponent|SetBeamSourceTangent (Variables|Default|GetPS_Lightning) (Math|Random|RandomIntegerinRange 0 (- (Class|ParticleSystemComponent|GetNumActiveParticles (Variables|Default|GetPS_Lightning)) 1)) (Math|Vector|MakeVector (Math|Random|RandomFloatinRange -3e+01 3e+01) (Math|Random|RandomFloatinRange -3e+01 3e+01) (Math|Random|RandomFloatinRange -3e+01 3e+01))))
        (:then_1
          (Utilities|FlowControl|Delay (Math|Random|RandomFloatinRange 0.1 0.5))
          (Class|ParticleSystemComponent|SetBeamTargetTangent (Variables|Default|GetPS_Lightning) (Math|Random|RandomIntegerinRange 0 (- (Class|ParticleSystemComponent|GetNumActiveParticles (Variables|Default|GetPS_Lightning)) 1)) (Math|Vector|MakeVector (Math|Random|RandomFloatinRange -3e+01 3e+01) (Math|Random|RandomFloatinRange -3e+01 3e+01) (Math|Random|RandomFloatinRange -3e+01 3e+01))))))
    (:then_1
      ;[1 1 1] Throw object
      (bind _targetlaunch (Variables|Throw|GetTargetLaunch)
        (:then
          (CallFunction|BuildSpline (/ (Transformation|GetDistanceTo _targetlaunch) 2.0))
          (Utilities|FlowControl|Sequence
            (:then_0
              (Utilities|FlowControl|DoOnce false
                (:Completed
                  (Collision|BindEventtoOnActorHit (Variables|Particle|Target|GetTarget) (EventDispatchers|CreateEvent :!event Custom|OnTargetHit)))))
            (:then_1
              (Components|Timeline|SetPlayRate (Variables|Default|GetMoveSpline) (/ 1.0 (Variables|Throw|GetDuration)))
              (bind _alpha (Timeline|MoveSpline Play)
                (:Update
                  (Variables|Throw|SetAlpha _alpha)
                  (Transformation|SetWorldLocation (Variables|Default|GetRootCapsule) (Spline|GetLocationatDistanceAlongSpline _spline (Math|Float|Lerp 0.0 (Spline|GetSplineLength _spline) (Variables|Throw|GetAlpha)) "World") false false))
                (:Finished
                  (Variables|Throw|SetTargetLaunch 0)
                  (Transformation|SetRelativeLocation (Variables|Default|GetRootCapsule) "0, 0, 0" false false)
                  (CallFunction|ResetDoOnceThrow)
                  (Components|Timeline|SetNewTime (Variables|Default|GetMoveSpline) 0.0))))))
        (:else)))))

(fn ConstructionScript)

(fn Grab
  (params (Target :type Actor%20Object%20Reference))
  (bind _output_get (Variables|Particle|Target|SetTarget Target))
  (Transformation|SetWorldLocation (Variables|Default|GetRootCapsule) (Transformation|GetActorLocation _output_get) false false)
  (bind _asprimitive_component (Utilities|Casting|CastToPrimitiveComponent (Variables|/Script/Engine.Actor|GetRootComponent (Variables|Particle|Target|GetTarget))))
  (LocalVariables|SetPrimitiveTarget _asprimitive_component)
  (Class|PhysicsConstraintComponent|SetConstrainedComponents (Variables|Default|GetPhysicsConstraint) (Variables|Default|GetRootCapsule) "None" (LocalVariables|GetPrimitiveTarget) "None")
  (Physics|SetSimulatePhysics (LocalVariables|GetPrimitiveTarget) true)
  (Transformation|SetRelativeLocation (Variables|Default|GetRootCapsule) "0, 0, 0" false false))

(fn Init
  (params (SourceMesh :type Skeletal%20Mesh%20Component%20Object%20Reference) (SocketSource :type Name) (Target :type Actor%20Object%20Reference))
  (Variables|Particle|Source|SetSourceMesh SourceMesh)
  (Variables|Particle|Source|SetSocketSource SocketSource)
  (Variables|Particle|Target|SetTarget Target))

(fn Throw
  (params (TargetToLaunchTo :type Actor%20Object%20Reference) (Keep/drop :type Boolean))
  (Variables|Particle|Target|GetTarget
    (:then
      (Variables|Throw|SetTargetLaunch TargetToLaunchTo)
      (Variables|Throw|SetKeep/drop Keep/drop))
    (:else)))

(fn BuildSpline
  (params (SplineSize :type Float%20%28single-precision%29))
  (Spline|ClearSplinePoints (Variables|Default|GetSpline) true)
  (for (_array_element _array_index) (Variables|Spline|GetSplinePoints)
    (LocalVariables|SetIndex _array_index)
    (Spline|AddSplinePoint (Variables|Default|GetSpline) (* _array_element SplineSize) "Local" true)
    (Spline|SetTangentatSplinePoint (Variables|Default|GetSpline) (LocalVariables|GetIndex) (* (Utilities|Array|Get(acopy) (Variables|Spline|GetSplineTangents) (LocalVariables|GetIndex)) SplineSize) "Local" true)))