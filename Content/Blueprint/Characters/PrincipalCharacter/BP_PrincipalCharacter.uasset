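; Player character Blueprint with third-person, camera-relative movement, jumping, sword attacks and clamped HP, with no logic yet at zero health.
; Vertical look blends camera rotation and spring arm offsets between a base preset and two others.
; Attack hold and release drive AnimBP_PrincipalCharacter.
; Sword overlap runs a sphere trace, whose hit DetectCollision uses to apply point damage once until ResetDamagesValues clears it.
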(event Custom|BeginOverlap%28Sword%29
  (params (OverlappedComponent :type Primitive%20Component%20Object%20Reference) (OtherActor :type Actor%20Object%20Reference) (OtherComp :type Primitive%20Component%20Object%20Reference) (OtherBodyIndex :type Integer) (bFromSweep :type Boolean) (SweepResult :type Hit%20Result%20Structure%20%28by%20ref%29))
  (bind _capsulesword (Variables|Default|GetCapsuleSword))
  (bind _returnvalue (Transformation|GetWorldLocation _capsulesword))
  ;[1 1 1] Attack collision
  (bind _output_get (Variables|Damages|SetOverlappedComp OtherComp))
  (if (Utilities|IsValid _output_get)
    (bind _outhit (Collision|SphereTraceForObjects _returnvalue _returnvalue 1.5e+02 (Utilities|Array|MakeArray "ObjectTypeQuery9") false 0 "ForDuration" true "(R=1.000000,G=0.000000,B=0.000000,A=1.000000)" "(R=0.000000,G=1.000000,B=0.000000,A=1.000000)" 1.0))
    (Variables|Damages|SetHitResults _outhit)))

(event EventBeginPlay
  ;[1 1 1] Begin play
  (Variables|Stats|Health|SetCurrentHP (Variables|Stats|Health|GetMaxHP)))

(event Game|Damage|EventAnyDamage
  (params (Damage :type Float%20%28single-precision%29) (DamageType :type Damage%20Type%20Object%20Reference) (InstigatedBy :type Controller%20Object%20Reference) (DamageCauser :type Actor%20Object%20Reference))
  ;[1 1 1] Damages
  (CallFunction|ManageHP Damage))

(event Input|ActionEvents|InputActionAttack
  (params (Key :type Key%20Structure))
  ;[1 1 1] Attack
  (:Pressed
    (Variables|/Game/Characters/PrincipalCharacter/Animation/AnimBP_PrincipalCharacter.AnimBP_PrincipalCharacter_C|SetHoldAttack (.AsAnim%20BP%20Principal%20Character (Utilities|Casting|CastToAnimBP_PrincipalCharacter (Components|SkeletalMesh|GetAnimInstance (Variables|Character|GetMesh)))) true))
  (:Released
    (CallFunction|Attack)))

(event Input|ActionEvents|InputActionJump
  (params (Key :type Key%20Structure))
  ;[1 1 1] Inputs
  (:Pressed
    (Character|Jump))
  (:Released
    (Character|StopJumping)))

(event Input|AxisEvents|InputAxisMoveForward
  (params (AxisValue :type Float%20%28single-precision%29))
  ;[1 1 1] Inputs
  (Variables|Controls|Character|SetLeftVerticalAxis AxisValue)
  (Pawn|Input|AddMovementInput (Math|Vector|GetForwardVector (Variables|Default|GetCamera)) (Variables|Controls|Character|GetLeftVerticalAxis) false)
  (if (!= (Variables|Controls|Character|GetLeftVerticalAxis) 0.0)
    (Transformation|SetWorldRotation (Variables|Character|GetMesh) (Math|Rotator|MakeRotator 0.0 0.0 (- (.yaw (Transformation|GetWorldRotation (Variables|Default|GetSpringArm))) (Class|KismetMathLibrary|DegAtan2 (Variables|Controls|Character|GetLeftVerticalAxis) (Variables|Controls|Character|GetLeftHorizontalAxis)))) false false)))

(event Input|AxisEvents|InputAxisMoveRight
  (params (AxisValue :type Float%20%28single-precision%29))
  ;[1 1 1] Inputs
  (Variables|Controls|Character|SetLeftHorizontalAxis AxisValue)
  (Pawn|Input|AddMovementInput (Math|Vector|GetRightVector (Variables|Default|GetCamera)) (Variables|Controls|Character|GetLeftHorizontalAxis) false)
  (if (!= (Variables|Controls|Character|GetLeftHorizontalAxis) 0.0)
    (Transformation|SetWorldRotation (Variables|Character|GetMesh) (Math|Rotator|MakeRotator 0.0 0.0 (- (.yaw (Transformation|GetWorldRotation (Variables|Default|GetSpringArm))) (Class|KismetMathLibrary|DegAtan2 (Variables|Controls|Character|GetLeftVerticalAxis) (Variables|Controls|Character|GetLeftHorizontalAxis)))) false false)))

(event Input|AxisEvents|InputAxisLookUp
  (params (AxisValue :type Float%20%28single-precision%29))
  ;[1 1 1] Inputs
  (Variables|Controls|Camera|SetRightVerticalAxis AxisValue)
  (CallFunction|SetVerticalViewRotation))

(event Input|AxisEvents|InputAxisTurn
  (params (AxisValue :type Float%20%28single-precision%29))
  ;[1 1 1] Inputs
  (bind _output_get (Variables|Controls|Camera|SetRightHorizontalAxis AxisValue))
  (Transformation|AddLocalRotation (Variables|Default|GetSpringArm) (Math|Rotator|MakeRotator 0.0 0.0 (* _output_get (Variables|Controls|Camera|GetHorizontalSensitivity))) false false))

(fn ConstructionScript)

(fn SetVerticalViewRotation
  (Utilities|FlowControl|Sequence
    (:then_0
      ;[1 1 1] Set camera settings index
      (Math|Float|CompareFloat (.z (Variables|/Script/Engine.SpringArmComponent|GetTargetOffset (Variables|Default|GetSpringArm))) (.z (.targetoffset (.Value (Utilities|Map|Find (Variables|Controls|Camera|GetCameraSettings) 0))))
        (:>
          (Variables|Controls|Camera|SetCurrentCameraSetting 2))
        (:==
          (Variables|Controls|Camera|SetCurrentCameraSetting 0))
        (:<
          (Variables|Controls|Camera|SetCurrentCameraSetting 1))))
    (:then_1
      ;[1 1 1] Set LerpAlpha
      (Variables|Controls|Camera|SetLerpAlpha (Math|Float|Clamp(Float) (+ (Variables|Controls|Camera|GetLerpAlpha) (* (Variables|Controls|Camera|GetRightVerticalAxis) (/ (Variables|Controls|Camera|GetVerticalSensitivity) 1e+02) (Math|Float|SelectFloat -1.0 1.0 (== (Utilities|GetObjectiveCameraSettings) 2)))))))
    (:then_2
      ;[1 1 1] Apply settings to Camera and SpringArm
      (Transformation|SetRelativeRotation (Variables|Default|GetCamera) (Math|Rotator|Lerp(Rotator) (.camerarotation (.Value (Utilities|Map|Find (Variables|Controls|Camera|GetCameraSettings) 0))) (.camerarotation (.Value (Utilities|Map|Find (Variables|Controls|Camera|GetCameraSettings) (Utilities|GetObjectiveCameraSettings)))) (Variables|Controls|Camera|GetLerpAlpha) true) false false)
      (Variables|/Script/Engine.SpringArmComponent|SetTargetOffset (Variables|Default|GetSpringArm) (Math|Vector|Lerp(Vector) (.targetoffset (.Value (Utilities|Map|Find (Variables|Controls|Camera|GetCameraSettings) 0))) (.targetoffset (.Value (Utilities|Map|Find (Variables|Controls|Camera|GetCameraSettings) (Utilities|GetObjectiveCameraSettings)))) (Variables|Controls|Camera|GetLerpAlpha)))
      (Variables|/Script/Engine.SpringArmComponent|SetSocketOffset (Variables|Default|GetSpringArm) (Math|Vector|Lerp(Vector) (.socketoffset (.Value (Utilities|Map|Find (Variables|Controls|Camera|GetCameraSettings) 0))) (.socketoffset (.Value (Utilities|Map|Find (Variables|Controls|Camera|GetCameraSettings) (Utilities|GetObjectiveCameraSettings)))) (Variables|Controls|Camera|GetLerpAlpha))))))

(fn ManageHP
  (params (InputPin :type Float%20%28single-precision%29))
  (bind _output_get (Variables|Stats|Health|SetCurrentHP (Math|Float|Clamp(Float) (- (Variables|Stats|Health|GetCurrentHP) InputPin) 0.0 (Variables|Stats|Health|GetMaxHP))))
  (if (== _output_get 0.0)
    _))

(fn Attack
  (params (ChosenAttack :type Anim%20Montage%20Object%20Reference))
  (bind _mesh (Variables|Character|GetMesh))
  (bind _returnvalue (Components|SkeletalMesh|GetAnimInstance _mesh))
  (bind _asanim_bp_principal_character (Utilities|Casting|CastToAnimBP_PrincipalCharacter _returnvalue))
  (Default|PlayAttackAnim _asanim_bp_principal_character (Variables|Stats|Attack|GetAttackCooldown))
  (Variables|/Game/Characters/PrincipalCharacter/Animation/AnimBP_PrincipalCharacter.AnimBP_PrincipalCharacter_C|SetHoldAttack _asanim_bp_principal_character false)
  (return true))

(fn DetectCollision
  (Collision|BindEventtoOnComponentBeginOverlap (Variables|Default|GetCapsuleSword) (EventDispatchers|CreateEvent :!event Custom|BeginOverlap%28Sword%29))
  (if (and (not (Variables|Damages|GetDamagesApplied)) (.bblockinghit (Variables|Damages|GetHitResults)))
    (Variables|Damages|SetDamagesApplied true)
    (Game|Damage|ApplyPointDamage (Components|GetOwner (Variables|Damages|GetOverlappedComp)) (Variables|Stats|Attack|GetDamages) (Transformation|GetActorLocation) (Variables|Damages|GetHitResults) (Pawn|GetController self) self)
    (return false)))

(fn GetHP
  (return (Variables|Stats|Health|GetCurrentHP) (Variables|Stats|Health|GetMaxHP)))

(fn ResetDamagesValues
  (EventDispatchers|UnbindallEventsfromOnComponentBeginOverlap (Variables|Default|GetCapsuleSword))
  (Variables|Damages|SetTouchedBone "None")
  (Variables|Damages|SetDamagesApplied false)
  (Variables|Damages|SetOverlappedComp 0)
  (Variables|Damages|SetHitResults "")
  (return true))