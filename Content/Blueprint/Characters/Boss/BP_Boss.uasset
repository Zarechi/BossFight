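; Boss character with separate arm and head health pools, routing point damage by bone-name suffix.
; A depleted arm ragdolls below its broken shoulder constraint, gains a grappling hook and advances the Blackboard phase, while a depleted head stops AI logic.
; BeginPlay already breaks the left arm this way.
; Attack functions filter DB_Attack rows through a body-part check and play montages through AnimBP_Boss with random cooldowns.
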(event OnComponentHit(Mesh)
  (params (HitComponent :type Primitive%20Component%20Object%20Reference) (OtherActor :type Actor%20Object%20Reference) (OtherComp :type Primitive%20Component%20Object%20Reference) (NormalImpulse :type Vector :default "0, 0, 0") (Hit :type Hit%20Result%20Structure%20%28by%20ref%29)))

(event EventBeginPlay
  ;[1 1 1] Begin play
  (Variables|Stats|Health|SetLeftArmHP (Variables|Stats|Health|GetLeftArmMaxHP))
  (Variables|Stats|Health|SetRightArmHP (Variables|Stats|Health|GetRightArmMaxHP))
  (Variables|Stats|Health|SetHeadHP (Variables|Stats|Health|GetHeadHP))
  (bind _grappelingtoset (CallFunction|BreakBone (Variables|Sockets|Skeleton|GetLeftShoulderSocket) (Variables|Sockets|Holder|GetLeftGrappelingSocket) (Variables|Sockets|Physics|GetLeftPhysicalSocketName) (Variables|Default|GetLeftGrappelingHolder)))
  (Variables|Components|SetLeftGrappeling _grappelingtoset))

(event EventTick
  (params (DeltaSeconds :type Float%20%28single-precision%29)))

(event Game|Damage|EventPointDamage
  (params (Damage :type Float%20%28single-precision%29) (DamageType :type Damage%20Type%20Object%20Reference) (HitLocation :type Vector :default "0, 0, 0") (HitNormal :type Vector :default "0, 0, 0") (HitComponent :type Primitive%20Component%20Object%20Reference) (BoneName :type Name :default "None") (ShotFromDirection :type Vector :default "0, 0, 0") (InstigatedBy :type Controller%20Object%20Reference) (DamageCauser :type Actor%20Object%20Reference) (HitInfo :type Hit%20Result%20Structure%20%28by%20ref%29))
  (CallFunction|ManageHP Damage (Utilities|String|ToString(Name) BoneName)))

(fn ConstructionScript)

(fn ManageHP
  (params (ValueToAdd :type Float%20%28single-precision%29) (TouchedSocket :type String))
  (Utilities|GetDamagedPart TouchedSocket
    (:LeftArm
      ;[1 1 1] Left arm
      (bind _output_get (Variables|Stats|Health|SetLeftArmHP (Math|Float|Clamp(Float) (- (Variables|Stats|Health|GetLeftArmHP) ValueToAdd) 0.0 (Variables|Stats|Health|GetLeftArmMaxHP))))
      (if (== _output_get 0.0)
        (CallFunction|BreakBone (Variables|Sockets|Skeleton|GetLeftShoulderSocket) (Variables|Sockets|Holder|GetLeftGrappelingSocket) "None")))
    (:RightArm
      ;[1 1 1] Right arm
      (bind _output_get_2 (Variables|Stats|Health|SetRightArmHP (Math|Float|Clamp(Float) (- (Variables|Stats|Health|GetRightArmHP) ValueToAdd) 0.0 (Variables|Stats|Health|GetRightArmMaxHP))))
      (if (== _output_get_2 0.0)
        (CallFunction|BreakBone (Variables|Sockets|Skeleton|GetRightShoulderSocket) (Variables|Sockets|Holder|GetRightGrappelingSocket) "None")))
    (:Head
      ;[1 1 1] Head
      (bind _output_get_3 (Variables|Stats|Health|SetHeadHP (Math|Float|Clamp(Float) (- (Variables|Stats|Health|GetHeadHP) ValueToAdd) 0.0 (Variables|Stats|Health|GetHeadMaxHP))))
      (if (== _output_get_3 0.0)
        (CallFunction|Death)))))

(fn BreakBone
  (params (SocketName :type Name) (GrappelingSocketName :type Name) (PhysicalSocketName :type Name) (Grappeling :type Child%20Actor%20Component%20Object%20Reference))
  (bind _childactor (Variables|/Script/Engine.ChildActorComponent|GetChildActor Grappeling))
  (bind _asbp_grappeling_hook (Utilities|Casting|CastToBP_GrappelingHook _childactor))
  (Class|SkeletalMeshComponent|SetAllBodiesBelowSimulatePhysics (Variables|Character|GetMesh) SocketName true true)
  (Class|SkeletalMeshComponent|SetAllBodiesBelowPhysicsBlendWeight (Variables|Character|GetMesh) SocketName 1.0 true true)
  (Class|SkeletalMeshComponent|BreakConstraint (Variables|Character|GetMesh) "0, 0, 0" "0, 0, 0" SocketName)
  (ChildActorComponent|SetChildActorClass Grappeling "/Game/Blueprint/Characters/PrincipalCharacter/BP_GrappelingHook.BP_GrappelingHook_C")
  (CallFunction|NextPhase)
  (Default|Init _asbp_grappeling_hook (Variables|Character|GetMesh) GrappelingSocketName)
  (return _asbp_grappeling_hook))

(fn Death
  (AI|Logic|StopLogic (Variables|/Script/AIModule.AIController|GetBrainComponent (AI|GetAIController self)) "Death"))

(fn NextPhase
  (Math|Integer|IncrementInt (Variables|Phases|GetCurrentPhase)
    (:%20%20
      (AI|Components|Blackboard|SetValueasBool (AI|GetBlackboard 0) (Utilities|String|StringToName "NewPhase?") true))))

(fn Attack
  (params (ChosenAttack :type Anim%20Montage%20Object%20Reference))
  (Default|PlayAttackMontage (.AsAnim%20BP%20Boss (Utilities|Casting|CastToAnimBP_Boss (Components|SkeletalMesh|GetAnimInstance (Variables|Character|GetMesh)))) ChosenAttack (Math|Random|RandomFloatinRange (Variables|Stats|Attack|GetMinAtkCooldown) (Variables|Stats|Attack|GetMaxAtkCooldown)))
  (return true))

(fn DetectCollision
  (return false))

(fn FindAllowedAttacks
  (Utilities|Map|Clear (Variables|Phases|GetAllowedAttacks))
  (bind _outrownames (DataTable|GetDataTableRowNames "/Game/Blueprint/DataTable/DB_Attack.DB_Attack"))
  (for _array_element _outrownames
    (bind _output_get (LocalVariables|SetCurrentRowName _array_element))
    (bind _returnvalue (Utilities|GetDataTableRow "/Game/Blueprint/DataTable/DB_Attack.DB_Attack" _output_get)
      (:then
        (if (Utilities|AttackCheck (.bodyparts _returnvalue))
          (Utilities|Map|Add (Variables|Phases|GetAllowedAttacks) (LocalVariables|GetCurrentRowName) 0.0)))))
  (return (Variables|Phases|GetAllowedAttacks)))

(fn GetAllowedAttacks
  (return (Variables|Phases|GetAllowedAttacks)))

(fn GetBossHP
  (return (Variables|Stats|Health|GetRightArmHP) (Variables|Stats|Health|GetLeftArmHP) (Variables|Stats|Health|GetHeadHP)))

(fn GetHP
  (return (+ (Variables|Stats|Health|GetLeftArmHP) (Variables|Stats|Health|GetRightArmHP) (Variables|Stats|Health|GetHeadHP)) (+ (Variables|Stats|Health|GetLeftArmMaxHP) (Variables|Stats|Health|GetRightArmMaxHP) (Variables|Stats|Health|GetHeadMaxHP))))

(fn ResetDamagesValues
  (return false))