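; Boss character with separate health for left arm, right arm and head, driven by a behavior tree.
; Point damage routes by bone-name suffix; a depleted arm calls BreakBone, and a depleted head stops the AI.
; BreakBone, also run on both shoulders at BeginPlay, ragdolls the limb, attaches a grappling hook and advances the Blackboard phase.
; Helpers filter data-table attacks, play montages, and handle grab/throw with decal feedback and random tag cooldowns.
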(event EventBeginPlay
  ;[1 1 1] Begin play
  (|CallParentFunction)
  (Variables|Stats|Health|SetLeftArmHP (Variables|Stats|Health|GetLeftArmMaxHP))
  (Variables|Stats|Health|SetRightArmHP (Variables|Stats|Health|GetRightArmMaxHP))
  (Variables|Stats|Health|SetHeadHP (Variables|Stats|Health|GetHeadMaxHP))
  (Variables|Default|SetMaxHP (+ (Variables|Stats|Health|GetLeftArmMaxHP) (Variables|Stats|Health|GetRightArmMaxHP) (Variables|Stats|Health|GetHeadMaxHP)))
  (Variables|Default|SetCurrentHP (+ (Variables|Stats|Health|GetLeftArmHP) (Variables|Stats|Health|GetRightArmHP) (Variables|Stats|Health|GetHeadHP)))
  (bind _grappelingtoset (CallFunction|BreakBone (Variables|Sockets|Skeleton|GetLeftShoulderSocket) (Variables|Sockets|Holder|GetLeftGrappelingSocket) (Variables|Default|GetLeftGrappelingHolder)))
  (Variables|Components|SetGrappeling _grappelingtoset)
  (bind _grappelingtoset_2 (CallFunction|BreakBone (Variables|Sockets|Skeleton|GetRightShoulderSocket) (Variables|Sockets|Holder|GetRightGrappelingSocket) (Variables|Default|GetLeftGrappelingHolder)))
  (Variables|Components|SetGrappeling _grappelingtoset_2))

(event EventTick
  (params (DeltaSeconds :type Float%20%28single-precision%29))
  (Rendering|Debug|DrawDebugPoint (Transformation|GetActorLocation (Variables|/Script/Engine.ChildActorComponent|GetChildActor (Variables|Default|GetTargetHolder))) 25.0 "(R=1.000000,G=0.000000,B=0.000000,A=1.000000)" 0.0))

(event Game|Damage|EventPointDamage
  (params (Damage :type Float%20%28single-precision%29) (DamageType :type Damage%20Type%20Object%20Reference) (HitLocation :type Vector :default "0, 0, 0") (HitNormal :type Vector :default "0, 0, 0") (HitComponent :type Primitive%20Component%20Object%20Reference) (BoneName :type Name :default "None") (ShotFromDirection :type Vector :default "0, 0, 0") (InstigatedBy :type Controller%20Object%20Reference) (DamageCauser :type Actor%20Object%20Reference) (HitInfo :type Hit%20Result%20Structure%20%28by%20ref%29))
  (CallFunction|ManageHP Damage (Utilities|String|ToString(Name) BoneName)))

(fn ConstructionScript)

(fn ManageHP
  (params (ValueToAdd :type Float%20%28single-precision%29) (TouchedSocket :type String))
  (Utilities|GetDamagedPart TouchedSocket
    (:LeftArm
      ;[1 1 1] Left arm
      (bind _output_get (Variables|Stats|Health|SetLeftArmHP (Math|Float|Clamp(Float) (- (Variables|Stats|Health|GetLeftArmHP) ValueToAdd) 0.0 (Variables|Stats|Health|GetLeftArmMaxHP))))
      (if (== _output_get 0.0)
        (bind _grappelingtoset (CallFunction|BreakBone (Variables|Sockets|Skeleton|GetLeftShoulderSocket) (Variables|Sockets|Holder|GetLeftGrappelingSocket) (Variables|Default|GetLeftGrappelingHolder)))
        (bind _grappeling (Variables|Components|GetGrappeling)
          (:then
            (Actor|DestroyActor _grappeling))
          (:else
            _))
        (Variables|Components|SetGrappeling _grappelingtoset)))
    (:RightArm
      ;[1 1 1] Right arm
      (bind _output_get_2 (Variables|Stats|Health|SetRightArmHP (Math|Float|Clamp(Float) (- (Variables|Stats|Health|GetRightArmHP) ValueToAdd) 0.0 (Variables|Stats|Health|GetRightArmMaxHP))))
      (if (== _output_get_2 0.0)
        (bind _grappelingtoset_2 (CallFunction|BreakBone (Variables|Sockets|Skeleton|GetRightShoulderSocket) (Variables|Sockets|Holder|GetRightGrappelingSocket) (Variables|Default|GetRightGrappelingHolder)))
        (bind _grappeling_2 (Variables|Components|GetGrappeling)
          (:then
            (Actor|DestroyActor _grappeling_2))
          (:else
            _))
        (Variables|Components|SetGrappeling _grappelingtoset_2)))
    (:Head
      (Development|PrintString (Utilities|String|Append "-" (Utilities|String|ToString(Float) ValueToAdd) " to head => " (Utilities|String|ToString(Float) (Variables|Stats|Health|GetHeadHP))))
      ;[1 1 1] Head
      (bind _output_get_3 (Variables|Stats|Health|SetHeadHP (Math|Float|Clamp(Float) (- (Variables|Stats|Health|GetHeadHP) ValueToAdd) 0.0 (Variables|Stats|Health|GetHeadMaxHP))))
      (if (== _output_get_3 0.0)
        (CallFunction|Death)))))

(fn BreakBone
  (params (SocketName :type Name) (GrappelingSocketName :type Name) (Grappeling :type Child%20Actor%20Component%20Object%20Reference))
  (bind _childactor (Variables|/Script/Engine.ChildActorComponent|GetChildActor Grappeling))
  (bind _asbp_grappeling_hook (Utilities|Casting|CastToBP_GrappelingHook _childactor))
  (Class|SkeletalMeshComponent|SetAllBodiesBelowSimulatePhysics (Variables|Character|GetMesh) SocketName true true)
  (Class|SkeletalMeshComponent|SetAllBodiesBelowPhysicsBlendWeight (Variables|Character|GetMesh) SocketName 1.0 true true)
  (Class|SkeletalMeshComponent|BreakConstraint (Variables|Character|GetMesh) "0, 0, 0" "0, 0, 0" SocketName)
  (ChildActorComponent|SetChildActorClass Grappeling "/Game/Blueprint/Characters/PrincipalCharacter/BP_GrappelingHook.BP_GrappelingHook_C")
  (CallFunction|NextPhase)
  (Default|Init _asbp_grappeling_hook (Variables|Character|GetMesh) GrappelingSocketName)
  (return _asbp_grappeling_hook))

(fn Death
  (AI|Logic|StopLogic (Variables|/Script/AIModule.AIController|GetBrainComponent (AI|GetAIController self)) "Death"))

(fn NextPhase
  (Math|Integer|IncrementInt (Variables|Phases|GetCurrentPhase)
    (:%20%20
      (AI|Components|Blackboard|SetValueasBool (AI|GetBlackboard 0) (Utilities|String|StringToName "NewPhase?") true))))

(fn SetCooldown
  (Class|BehaviorTreeComponent|AddCooldownTagDuration (.AsBehavior%20Tree%20Component (Utilities|Casting|CastToBehaviorTreeComponent (Variables|/Script/AIModule.AIController|GetBrainComponent (AI|GetAIController self)))) "(TagName=\"Boss.Attack\")" (Math|Random|RandomFloatinRange (Variables|Default|GetMinAtkCD) (Variables|Default|GetMaxAtkCD)) false))

(fn DecalFeedback
  (params (TargetLocation :type Vector))
  (bind _returnvalue (Game|SpawnActorfromClass "/Script/Engine.DecalActor" (Math|Transform|MakeTransform TargetLocation "0, 0, 0" "1,1,1") "Undefined" 0 0))
  (bind _output_get (LocalVariables|SetDecalActor _returnvalue))
  (Transformation|SetWorldRotation (Variables|/Script/Engine.DecalActor|GetDecal _output_get) "90.0,0.0,0.0" false false)
  (Rendering|Components|Decal|SetDecalMaterial (Variables|/Script/Engine.DecalActor|GetDecal (LocalVariables|GetDecalActor)) "/Game/Blueprint/Characters/Boss/Decals/M_Decal_Inst.M_Decal_Inst")
  (return (LocalVariables|GetDecalActor)))

(fn Attack
  (params (ChosenAttack :type Anim%20Montage%20Object%20Reference))
  (Default|PlayAttackMontage (.AsAnim%20BP%20Boss (Utilities|Casting|CastToAnimBP_Boss (Components|SkeletalMesh|GetAnimInstance (Variables|Character|GetMesh)))) ChosenAttack)
  (return true))

(fn GetBossHP
  (return (Utilities|Map|MakeMap "LeftArm" (Variables|Stats|Health|GetLeftArmHP) "RightArm" (Variables|Stats|Health|GetRightArmHP) "Head" (Variables|Stats|Health|GetHeadHP))))

(fn FindAllowedAttacks
  (Utilities|Map|Clear (Variables|Default|GetAllowedAttacks))
  (bind _outrownames (DataTable|GetDataTableRowNames "/Game/Blueprint/DataTable/DB_Attack.DB_Attack"))
  (for _array_element _outrownames
    (bind _output_get (LocalVariables|SetCurrentRowName _array_element))
    (bind _returnvalue (Utilities|GetDataTableRow "/Game/Blueprint/DataTable/DB_Attack.DB_Attack" _output_get)
      (:then
        (if (Utilities|AttackCheck (.bodyparts _returnvalue))
          (Utilities|Map|Add (Variables|Default|GetAllowedAttacks) (LocalVariables|GetCurrentRowName) 0.0)))))
  (return (Variables|Default|GetAllowedAttacks)))

(fn GetGrappeling
  (return (Variables|Components|GetGrappeling)))

(fn Grab
  (params (TargetGrab :type Actor%20Object%20Reference) (TargetAim :type Actor%20Object%20Reference))
  (Utilities|Casting|CastToCharacter TargetGrab
    (:then
      (Default|Grab (Variables|Components|GetGrappeling) TargetGrab (Variables|/Script/Engine.ChildActorComponent|GetChildActor (Variables|Default|GetTargetHolder))))
    (:CastFailed
      (bind _output_get (Variables|Phases|SetHasObject (not (Utilities|IsValid TargetAim))))
      (if _output_get
        _
        (else
          (CallFunction|DecalFeedback (Transformation|GetActorLocation TargetAim))))
      (Default|Grab (Variables|Components|GetGrappeling) TargetGrab TargetAim)
      (Utilities|Time|SetTimerbyFunctionName self "SetCooldown" 0.2)
      (return true))))

(fn HasObjectinGrappeling
  (return (Variables|Phases|GetHasObject)))

(fn Throw
  (params (TargetAim :type Actor%20Object%20Reference) (KeepOrDrop :type Boolean))
  (Variables|Phases|SetHasObject KeepOrDrop)
  (bind _decal (CallFunction|DecalFeedback (Transformation|GetActorLocation TargetAim)))
  (Default|Throw (Variables|Components|GetGrappeling) TargetAim KeepOrDrop _decal)
  (Utilities|Time|SetTimerbyFunctionName self "SetCooldown" 0.2)
  (return true))