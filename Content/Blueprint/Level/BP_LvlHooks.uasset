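; BP_LvlHooks is a level actor that joins a Source and a Target actor with a physics constraint and a lightning beam.
; SetLink, run on construction and BeginPlay, constrains the Source root to the Target's skeletal mesh (or root) at named bones, then moves itself to the Source.
; Tick pins the beam endpoints to both actors and randomly wiggles emitter tangents after short delays.
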(event EventBeginPlay
  (CallFunction|SetLink))

(event EventTick
  (params (DeltaSeconds :type Float%20%28single-precision%29))
  (for _index (range 0 (- (Class|ParticleSystemComponent|GetNumActiveParticles (Variables|Default|GetPS_Lightning)) 1))
    ;[1 1 1] Set Source and Target
    (Variables|Link|Default|SetParticleIndex _index)
    (Class|ParticleSystemComponent|SetBeamSourcePoint (Variables|Default|GetPS_Lightning) (Variables|Link|Default|GetParticleIndex) (Transformation|GetActorLocation (Variables|Link|Source|GetSource)))
    (Variables|Link|Target|SetTargetPoint (Transformation|GetActorLocation (Variables|Link|Target|GetTarget)))
    (Class|ParticleSystemComponent|SetBeamTargetPoint (Variables|Default|GetPS_Lightning) (Variables|Link|Default|GetParticleIndex) (Variables|Link|Target|GetTargetPoint)))
  ;[1 1 1] Wiggle beam tangent
  (Utilities|FlowControl|Sequence
    (:then_0
      (Utilities|FlowControl|Delay (Math|Random|RandomFloatinRange 0.1 0.5))
      (Class|ParticleSystemComponent|SetBeamSourceTangent (Variables|Default|GetPS_Lightning) (Math|Random|RandomIntegerinRange 0 (- (Class|ParticleSystemComponent|GetNumActiveParticles (Variables|Default|GetPS_Lightning)) 1)) (Math|Vector|MakeVector (Math|Random|RandomFloatinRange -3e+01 3e+01) (Math|Random|RandomFloatinRange -3e+01 3e+01) (Math|Random|RandomFloatinRange -3e+01 3e+01))))
    (:then_1
      (Utilities|FlowControl|Delay (Math|Random|RandomFloatinRange 0.1 0.5))
      (Class|ParticleSystemComponent|SetBeamTargetTangent (Variables|Default|GetPS_Lightning) (Math|Random|RandomIntegerinRange 0 (- (Class|ParticleSystemComponent|GetNumActiveParticles (Variables|Default|GetPS_Lightning)) 1)) (Math|Vector|MakeVector (Math|Random|RandomFloatinRange -3e+01 3e+01) (Math|Random|RandomFloatinRange -3e+01 3e+01) (Math|Random|RandomFloatinRange -3e+01 3e+01))))))

(fn ConstructionScript
  (CallFunction|SetLink))

(fn SetLink
  (bind _target (Variables|Link|Target|GetTarget))
  (bind _returnvalue (Actor|GetComponentsByClass _target "/Script/Engine.SkeletalMeshComponent"))
  (bind _asprimitive_component (Utilities|Casting|CastToPrimitiveComponent (Variables|/Script/Engine.Actor|GetRootComponent (Variables|Link|Source|GetSource))))
  (LocalVariables|SetPrimitiveSource _asprimitive_component)
  (bind _asprimitive_component_2 (Utilities|Casting|CastToPrimitiveComponent (Utilities|SelectObject (Variables|/Script/Engine.Actor|GetRootComponent _target) (Utilities|Array|Get(acopy) _returnvalue) (== (Utilities|Array|Length _returnvalue) 0))))
  (LocalVariables|SetPrimitiveTarget _asprimitive_component_2)
  (Class|PhysicsConstraintComponent|SetConstrainedComponents (Variables|Default|GetPhysicsConstraint) (LocalVariables|GetPrimitiveSource) (Variables|Link|Source|GetSourceBoneName) (LocalVariables|GetPrimitiveTarget) (Variables|Link|Target|GetTargetBoneName))
  (Transformation|SetActorLocation (Transformation|GetWorldLocation (LocalVariables|GetPrimitiveSource)) false false))