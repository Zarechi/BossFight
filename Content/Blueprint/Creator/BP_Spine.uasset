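; BP_Spine builds a spine along a spline at BeginPlay, as evenly spaced static meshes joined by spline mesh segments.
; CreateSpine places the meshes at fixed distance intervals, then rebuilds the spline from their locations plus the original endpoints.
; CreateSpineSplineMesh then adds a spline mesh between each pair of new points, using their locations and tangents.
; The construction script is empty, so nothing is generated in the editor.
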(event EventBeginPlay
  (CallFunction|CreateSpine (Variables|Default|GetSpacing) (Variables|Default|GetMesh) (Variables|Default|GetMaterial))
  (CallFunction|CreateSpineSplineMesh))

(fn ConstructionScript)

(fn CreateSpineSplineMesh
  (for _index (range 0 (- (Spline|GetNumberOfSplinePoints (Variables|Default|GetSpline)) 2))
    (LocalVariables|SetIndex _index)
    (bind _returnvalue (AddComponent|AddSplineMeshComponent true (Transformation|GetActorTransform)))
    (bind _output_get (LocalVariables|SetCreatedSplineMesh _returnvalue))
    (Rendering|Material|SetMaterial _output_get 0 (Variables|Default|GetSplineMeshMaterial))
    (Transformation|AttachComponentToComponent (LocalVariables|GetCreatedSplineMesh) (Variables|Transformation|GetRootComponent) "None" "KeepWorld" "KeepWorld" "KeepWorld" true)
    (SplineMesh|SetStartandEnd (LocalVariables|GetCreatedSplineMesh) (.Location (Spline|GetLocationandTangentatSplinePoint (Variables|Default|GetSpline) (LocalVariables|GetIndex) "Local")) (.Tangent (Spline|GetLocationandTangentatSplinePoint (Variables|Default|GetSpline) (LocalVariables|GetIndex) "Local")) (.Location (Spline|GetLocationandTangentatSplinePoint (Variables|Default|GetSpline) (+ (LocalVariables|GetIndex) 1) "Local")) (.Tangent (Spline|GetLocationandTangentatSplinePoint (Variables|Default|GetSpline) (+ (LocalVariables|GetIndex) 1) "Local")) true :!class /Script/Engine.SplineMeshComponent)))

(fn CreateSpine
  (params (SpaceBetweenMesh :type Float%20%28single-precision%29) (AppliedMesh :type Static%20Mesh%20Object%20Reference) (AppliedMaterial :type Material%20Interface%20Object%20Reference))
  (bind _spline (Variables|Default|GetSpline))
  (Utilities|Array|Add (LocalVariables|GetAllMeshesLocation) (Spline|GetLocationatSplinePoint (Variables|Default|GetSpline) 0 "World"))
  (for _index (range 0 (.ReturnValue (Math|Float|Division(WholeandRemainder) (Spline|GetSplineLength (Variables|Default|GetSpline)) SpaceBetweenMesh)))
    (bind _output_get (LocalVariables|SetIndex _index))
    (bind _returnvalue (AddComponent|AddStaticMeshComponent true (Spline|GetTransformatDistanceAlongSpline (Variables|Default|GetSpline) (* _output_get SpaceBetweenMesh) "World" true)))
    (bind _output_get_2 (LocalVariables|SetCreatedMesh _returnvalue))
    (Components|StaticMesh|SetStaticMesh _output_get_2 AppliedMesh)
    (Rendering|Material|SetMaterial (LocalVariables|GetCreatedMesh) 0 AppliedMaterial)
    (Utilities|Array|Add (LocalVariables|GetAllMeshesLocation) (Transformation|GetWorldLocation (LocalVariables|GetCreatedMesh))))
  (Utilities|Array|Add (LocalVariables|GetAllMeshesLocation) (Spline|GetLocationatSplinePoint _spline (Spline|GetNumberOfSplinePoints _spline) "World"))
  (Spline|SetSplinePoints (Variables|Default|GetSpline) (LocalVariables|GetAllMeshesLocation) "World" true))