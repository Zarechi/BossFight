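; Custom camera Blueprint that hides static mesh actors blocking the line between its spring arm and camera.
; Each tick a Visibility trace finds the blocker, stores it as HiddenActor and hides it, then runs IsInViewport.
; That check projects mesh vertices, scaled but not translated or rotated, to screen bounds and draws debug points.
; Nothing acts on its result, so hidden actors are never shown again.
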(event EventTick
  (params (DeltaSeconds :type Float%20%28single-precision%29))
  (Utilities|FlowControl|Sequence
    (:then_0
      (bind _outhit (Collision|LineTraceByChannel (Transformation|GetWorldLocation (Variables|Default|GetSpringArm)) (Transformation|GetWorldLocation (Variables|Default|GetCamera)) "TraceTypeQuery1" false 0 "None"))
      (if (.bBlockingHit (Collision|BreakHitResult _outhit))
        (bind _asstatic_mesh_actor (Utilities|Casting|CastToStaticMeshActor (.HitActor (Collision|BreakHitResult _outhit))))
        (bind _output_get (Variables|Default|SetHiddenActor _asstatic_mesh_actor))
        (Rendering|SetActorHiddenInGame _output_get true)))
    (:then_1
      (Variables|Default|GetHiddenActor
        (:then
          (Utilities|IsinViewport?))
        (:else)))))

(fn ConstructionScript)